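; Player Blueprint that shows and removes a lock-on marker for a targeted boss.
; The UpdateLockonWBP callback stores the target and, when locking on, spawns a BP_TargetLockOnUI actor slightly above it, then snaps it to the boss mesh's neck_01 socket.
; On unlock or an invalid target, it destroys the spawned marker and clears its reference.
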(event EventBeginPlay)

(event Collision|EventActorBeginOverlap
  (params (OtherActor :type Actor%20Object%20Reference)))

(event EventTick
  (params (DeltaSeconds :type Float%20%28single-precision%29)))

(event EventUpdateLockonWBP
  (params (bIsLockOn :type Boolean) (targetBoss :type %20Object%20Reference))
  ;[1 1 1] UI Update CallBack Event for Lock On to target
  (Variables|Default|SetTarget%20Boss targetBoss)
  (if bIsLockOn
    (Utilities|IsValid (Variables|Default|GetTarget%20Boss)
      (:Is%20Valid
        (bind _returnvalue (Game|SpawnActorfromClass "/Game/Blueprints/Player/BP_TargetLockOnUI.BP_TargetLockOnUI_C" (Math|Transform|MakeTransform (Math|Vector|MakeVector (.x (.location (Transformation|GetActorTransform (Variables|Default|GetTarget%20Boss)))) (.y (.location (Transformation|GetActorTransform (Variables|Default|GetTarget%20Boss)))) (+ (.z (.location (Transformation|GetActorTransform (Variables|Default|GetTarget%20Boss)))) 2e+01)) (.rotation (Transformation|GetActorTransform (Variables|Default|GetTarget%20Boss))) (.scale (Transformation|GetActorTransform (Variables|Default|GetTarget%20Boss)))) "AlwaysSpawn" "MultiplyWithRoot" 0 0))
        (bind _output_get (Variables|Default|SetSpawnedUI _returnvalue))
        (Transformation|AttachComponentToComponent _output_get (Variables|/Script/Engine.Character|GetMesh (Variables|Default|GetTarget%20Boss)) "neck_01" "SnapToTarget" "SnapToTarget" "SnapToTarget" true))
      (:Is%20Not%20Valid
        (Utilities|IsValid (Variables|Default|GetSpawnedUI) :!label _label
          (:Is%20Valid
            (Actor|DestroyActor (Variables|Default|GetSpawnedUI))
            (Variables|Default|SetSpawnedUI 0)))))
    (else
      (goto _label))))

(fn ConstructionScript)